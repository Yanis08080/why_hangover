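; TriggerAfterKeys is a trigger actor that gates a level sequence on all collectibles being gathered.
; Its Suuu overlap component enables the actor's input while BP_ThirdPersonCharacterV2 is inside and disables it on exit.
; Pressing E checks that CollectibleLeft on BP_TopDownGameMode is zero, then creates a level sequence player; no Play call or sequence asset is shown.
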(event `Key|E`
  (params (Key :type "Key Structure"))
  (:`Pressed`
    (bind _asbp_top_down_game_mode (cast `/Game/TopDown/Blueprints/BP_TopDownGameMode` (`GameplayStatics.GetGameMode`)))
    (if (== (`/Game/TopDown/Blueprints/BP_TopDownGameMode.Collectible_Left` _asbp_top_down_game_mode) 0)
      (`LevelSequencePlayer.CreateLevelSequencePlayer` null))))

(event `self.Suuu.OnComponentBeginOverlap`
  (params (OverlappedComponent :type "PrimitiveComponent Object Reference") (OtherActor :type "Actor Object Reference") (OtherComp :type "PrimitiveComponent Object Reference") (OtherBodyIndex :type Integer) (bFromSweep :type Boolean) (SweepResult :type "HitResult Structure (by ref)"))
  (cast `/Game/Yanis/Camera_Setup/Blueprints/BP_ThirdPersonCharacterV2` OtherActor)
  (`self.EnableInput` (`GameplayStatics.GetPlayerController` 0)))

(event `self.Suuu.OnComponentEndOverlap`
  (params (OverlappedComponent :type "PrimitiveComponent Object Reference") (OtherActor :type "Actor Object Reference") (OtherComp :type "PrimitiveComponent Object Reference") (OtherBodyIndex :type Integer))
  (cast `/Game/Yanis/Camera_Setup/Blueprints/BP_ThirdPersonCharacterV2` OtherActor)
  (`self.DisableInput` (`GameplayStatics.GetPlayerController` 0)))

(fn `UserConstructionScript`)