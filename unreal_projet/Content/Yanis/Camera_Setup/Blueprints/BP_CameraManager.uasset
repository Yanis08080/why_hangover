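; BP_CameraManager tracks which camera is active and handles switching to a new one.
; SetActiveCamera ignores a request for the already active camera, otherwise it stores any valid current camera as the previous one and takes the new one.
; It then enables the new camera's tick, broadcasts OnCameraChanged with both cameras, and snaps the active camera to its offset location and character view.
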(fn `SetActiveCamera`
  (params (NewActiveCamera :type "/Game/Yanis/Camera_Setup/Blueprints/BP_MasterCamera Object Reference"))
  (bind _currentactivecamera (`self.CurrentActiveCamera`))
  (`/Engine/EditorBlueprintResources/StandardMacros.IsValid` _currentactivecamera
    (:`Is Valid`
      (if (!= NewActiveCamera _currentactivecamera)
        (set `self.PreviousCamera` (`self.CurrentActiveCamera`))
        (set `self.CurrentActiveCamera` NewActiveCamera :!label _label)
        (`self.SetActorTickEnabled` NewActiveCamera true)
        (`self.OnCameraChanged` (`self.PreviousCamera`) (`self.CurrentActiveCamera`))
        (`|ExecutionSequence`
          (:`then_0`
            (`/Game/Yanis/Camera_Setup/Blueprints/BP_MasterCamera.SnapToOffsetLoc` (`self.CurrentActiveCamera`)))
          (:`then_1`
            (`/Game/Yanis/Camera_Setup/Blueprints/BP_MasterCamera.SnapToCharacterView` (`self.CurrentActiveCamera`))))))
    (:`Is Not Valid`
      (goto _label))))

(fn `UserConstructionScript`)