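; Master camera actor that can follow the player along a spline rail, rotate to track them, or both.
; On BeginPlay it finds BP_CameraManager, optionally becomes the level's starting view, and keeps either the standard or cine camera component by type.
; While it is the manager's active camera, Tick moves RailPivot with speed-limited, interpolated rail motion and smoothed look-at, otherwise disabling itself.
; Snap functions place or aim the pivot instantly.
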(event `self.ReceiveBeginPlay`
  (`|ExecutionSequence`
    (:`then_0`
      (bind _returnvalue (`GameplayStatics.GetActorOfClass` "/Game/Yanis/Camera_Setup/Blueprints/BP_CameraManager.BP_CameraManager_C"))
      (`/Engine/EditorBlueprintResources/StandardMacros.IsValid` _returnvalue
        (:`Is Valid`
          (set `self.CameraManagerReference` _returnvalue))
        (:`Is Not Valid`
          (`KismetSystemLibrary.PrintString` "ERROR: No camera manager found in scene!!" true true (struct :`R` 1.0 :`A` 1.0)))))
    (:`then_1`
      (if (`self.bIsLevelStartCam`)
        (`PlayerController.SetViewTargetWithBlend` (`GameplayStatics.GetPlayerController` 0) self 0.0 "VTBlend_Linear" 0.0 false)
        (`/Game/Yanis/Camera_Setup/Blueprints/BP_CameraManager.SetActiveCamera` (`self.CameraManagerReference`) self)
        (if (`self.bIsTrackingCam`)
          (`self.SnapToCharacterView`))))
    (:`then_2`
      (`self.SwitchCamera` (`self.CameraTypes`)))))

(event `self.ReceiveTick`
  (params (DeltaSeconds :type "Float (single-precision)"))
  (set `self.Delta Seconds` DeltaSeconds)
  (if (== self (`/Game/Yanis/Camera_Setup/Blueprints/BP_CameraManager.CurrentActiveCamera` (`self.CameraManagerReference`)))
    (`|ExecutionSequence`
      (:`then_0`
        (`self.UpdateOnRailCamera`))
      (:`then_1`
        (`self.UpdateTrackingCamera`)))
    (else
      ; No ? Then disable tick
      (`self.SetActorTickEnabled` self false))))

(fn `SnapToCharacterView`
  (bind _railpivot (`self.RailPivot`))
  (if (`self.bIsTrackingCam`)
    (`SceneComponent.K2_SetWorldRotation` _railpivot (`KismetMathLibrary.FindLookAtRotation` (`SceneComponent.K2_GetComponentLocation` _railpivot) (`self.K2_GetActorLocation` (`GameplayStatics.GetPlayerCharacter` 0))) false false)))

(fn `SnapToOffsetLoc`
  (bind _spline (`self.Spline`))
  ; On rail cam enabled
  (if (`self.bIsOnRailCam`)
    (set `self.CurrentRailDistance` (`KismetMathLibrary.FClamp` (+ (`SplineComponent.GetDistanceAlongSplineAtSplineInputKey` _spline (`SplineComponent.FindInputKeyClosestToWorldLocation` _spline (`self.K2_GetActorLocation` (`GameplayStatics.GetPlayerCharacter` 0)))) (`self.FollowOffsetDistance`)) 0.0 (`SplineComponent.GetSplineLength` (`self.Spline`))))
    (`SceneComponent.K2_SetWorldLocation` (`self.RailPivot`) (`SplineComponent.GetLocationAtDistanceAlongSpline` (`self.Spline`) (`KismetMathLibrary.FClamp` (+ (`self.CurrentRailDistance`) (`self.LookAheadDistance`)) 0.0 (`SplineComponent.GetSplineLength` (`self.Spline`))) "World") false false)))

(fn `SwitchCamera`
  (params (Selection :type Byte :default 0))
  (switch `|SwitchEnum` (`self.CameraTypes`)
    (:`NewEnumerator0`
      (`ActorComponent.K2_DestroyComponent` (`self.CineCamera`)))
    (:`NewEnumerator1`
      (`ActorComponent.K2_DestroyComponent` (`self.Camera`)))))

(fn `UpdateOnRailCamera`
  (bind _spline (`self.Spline`))
  (bind _returnvalue (* (`self.DistanceFollowSpeed`) (`self.Delta Seconds`)))
  (bind _returnvalue_2 (`KismetMathLibrary.FClamp` (+ (`SplineComponent.GetDistanceAlongSplineAtSplineInputKey` _spline (`SplineComponent.FindInputKeyClosestToWorldLocation` _spline (`self.K2_GetActorLocation` (`GameplayStatics.GetPlayerCharacter` 0)))) (`self.FollowOffsetDistance`)) 0.0 (`SplineComponent.GetSplineLength` (`self.Spline`))))
  (bind _returnvalue_3 (- _returnvalue_2 (`self.CurrentRailDistance`)))
  ; On rail cam enabled
  (if (`self.bIsOnRailCam`)
    (set `self.CurrentRailDistance` (`KismetMathLibrary.FClamp` (`KismetMathLibrary.SelectFloat` _returnvalue_2 (+ (`self.CurrentRailDistance`) (* (`KismetMathLibrary.SignOfFloat` _returnvalue_3) _returnvalue)) (<= (`KismetMathLibrary.Abs` _returnvalue_3) _returnvalue)) 0.0 (`SplineComponent.GetSplineLength` (`self.Spline`))))
    (`SceneComponent.K2_SetWorldLocation` (`self.RailPivot`) (`KismetMathLibrary.VInterpTo` (`SceneComponent.K2_GetComponentLocation` (`self.RailPivot`)) (`SplineComponent.GetLocationAtDistanceAlongSpline` (`self.Spline`) (`KismetMathLibrary.FClamp` (+ (`self.CurrentRailDistance`) (`self.LookAheadDistance`)) 0.0 (`SplineComponent.GetSplineLength` (`self.Spline`))) "World") (`self.Delta Seconds`) (`self.FollowInterpSpeed`)) false false)))

(fn `UpdateTrackingCamera`
  ; Check if tracking enabled, if not, do nothing
  (if (`self.bIsTrackingCam`)
    ; Set current camera rotation
    (set `self.CurrentCameraRotation` (`SceneComponent.K2_GetComponentRotation` (`self.RailPivot`)))
    ; Rotate the camera
    (`SceneComponent.K2_SetWorldRotation` (`self.RailPivot`) (`KismetMathLibrary.RInterpTo` (`self.CurrentCameraRotation`) (`KismetMathLibrary.FindLookAtRotation` (`SceneComponent.K2_GetComponentLocation` (`self.RailPivot`)) (`self.K2_GetActorLocation` (`GameplayStatics.GetPlayerCharacter` 0))) (`self.Delta Seconds`) (`self.RotationInterpSpeed`)) false false)))

(fn `UserConstructionScript`)