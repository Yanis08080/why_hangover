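; BP_InspectableActor is a collectible world object that the player picks up by pressing E while nearby.
; Overlap of its Cube by BP_ThirdPersonCharacterV2 toggles the actor's input from player controller 0.
; Pressing E decrements CollectibleLeft on BP_TopDownGameMode, then destroys the actor.
; CanInspect always returns true and GetInspectMesh returns its StaticMesh, exposing it for inspection.
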(event `Key|E`
  (params (Key :type "Key Structure"))
  (:`Pressed`
    (bind _asbp_top_down_game_mode (cast `/Game/TopDown/Blueprints/BP_TopDownGameMode` (`GameplayStatics.GetGameMode`)))
    (bind _result (`/Engine/EditorBlueprintResources/StandardMacros.DecrementInt` (`/Game/TopDown/Blueprints/BP_TopDownGameMode.Collectible_Left` _asbp_top_down_game_mode))
      (:`  `
        (set `/Game/TopDown/Blueprints/BP_TopDownGameMode.Collectible_Left` _result _asbp_top_down_game_mode)
        (`self.K2_DestroyActor`)))))

(event `self.Cube.OnComponentBeginOverlap`
  (params (OverlappedComponent :type "PrimitiveComponent Object Reference") (OtherActor :type "Actor Object Reference") (OtherComp :type "PrimitiveComponent Object Reference") (OtherBodyIndex :type Integer) (bFromSweep :type Boolean) (SweepResult :type "HitResult Structure (by ref)"))
  (cast `/Game/Yanis/Camera_Setup/Blueprints/BP_ThirdPersonCharacterV2` OtherActor)
  (`self.EnableInput` (`GameplayStatics.GetPlayerController` 0)))

(event `self.Cube.OnComponentEndOverlap`
  (params (OverlappedComponent :type "PrimitiveComponent Object Reference") (OtherActor :type "Actor Object Reference") (OtherComp :type "PrimitiveComponent Object Reference") (OtherBodyIndex :type Integer))
  (cast `/Game/Yanis/Camera_Setup/Blueprints/BP_ThirdPersonCharacterV2` OtherActor)
  (`self.DisableInput` (`GameplayStatics.GetPlayerController` 0)))

(fn `CanInspect`
  (returns (CanInspect :type Boolean))
  (return true))

(fn `GetInspectMesh`
  (returns (GetStaticMesh :type "StaticMeshComponent Object Reference"))
  (return (`self.StaticMesh`)))

(fn `UserConstructionScript`)