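; Camera trigger volume that blends the player's view between an enter camera and an exit camera as the player crosses a line inside it.
; While the player overlaps the box, a looping timer runs, created once and then paused or unpaused on exit and re-entry.
; Each tick dots the player's direction against the line's forward vector, switching on a side change beyond a minimum gap.
; Switches also update the active camera on BP_CameraManager.
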(event `self.ReceiveBeginPlay`
  (bind _returnvalue (`GameplayStatics.GetActorOfClass` "/Game/Yanis/Camera_Setup/Blueprints/BP_CameraManager.BP_CameraManager_C"))
  (`/Engine/EditorBlueprintResources/StandardMacros.IsValid` _returnvalue
    (:`Is Valid`
      (set `self.CameraManagerReference` _returnvalue))
    (:`Is Not Valid`
      (`KismetSystemLibrary.PrintString` "ERROR: No camera manager found in scene!!" true true (struct :`R` 1.0 :`A` 1.0)))))

(event `Timer`
  (bind _line (`self.Line`))
  (bind _entercamera (`self.EnterCamera`))
  (bind _exitcamera (`self.ExitCamera`))
  (bind _returnvalue (`KismetMathLibrary.Dot_VectorVector` (`KismetMathLibrary.Normal` (- (`self.K2_GetActorLocation` (`GameplayStatics.GetPlayerPawn` 0)) (`SceneComponent.K2_GetComponentLocation` _line))) (`SceneComponent.GetForwardVector` _line)))
  (bind _returnvalue_2 (`KismetMathLibrary.SignOfFloat` _returnvalue))
  (bind _returnvalue_3 (<= _returnvalue_2 0.0))
  (if (and (!= _returnvalue_2 (`self.PreviousSide`)) (> (`KismetMathLibrary.Abs` _returnvalue) (`self.MinPlaneGap`)))
    ; Set previous side to be current side
    (set `self.PreviousSide` _returnvalue_2)
    (`KismetSystemLibrary.PrintString` (`KismetMathLibrary.SelectString` "Entering" "Exiting" _returnvalue_3) false)
    ; Check if entering or exiting
    (if _returnvalue_3
      ; Switch view to enter cam
      (`PlayerController.SetViewTargetWithBlend` (`GameplayStatics.GetPlayerController` 0) _entercamera (`self.Blend Time_ENTER`) "VTBlend_Linear" 0.0 false)
      (`/Game/Yanis/Camera_Setup/Blueprints/BP_CameraManager.SetActiveCamera` (`self.CameraManagerReference`) _entercamera)
      (else
        ; Switch view to exit cam
        (`PlayerController.SetViewTargetWithBlend` (`GameplayStatics.GetPlayerController` 0) _exitcamera (`self.Blend Time_EXIT`) "VTBlend_Linear" 0.0 false)
        (`/Game/Yanis/Camera_Setup/Blueprints/BP_CameraManager.SetActiveCamera` (`self.CameraManagerReference`) _exitcamera)))))

(event `self.Box.OnComponentBeginOverlap`
  (params (OverlappedComponent :type "PrimitiveComponent Object Reference") (OtherActor :type "Actor Object Reference") (OtherComp :type "PrimitiveComponent Object Reference") (OtherBodyIndex :type Integer) (bFromSweep :type Boolean) (SweepResult :type "HitResult Structure (by ref)"))
  ; Check we've ovelapped with player (Je sais pas comment traduire)
  (if (`self.IsPlayerActor ?` OtherActor)
    ; Le timer existe t'il deja
    (if (`KismetSystemLibrary.K2_IsValidTimerHandle` (`self.Timer Handle`))
      ; Si oui, sort de la pause
      (`KismetSystemLibrary.K2_UnPauseTimerHandle` (`self.Timer Handle`))
      (else
        ; Si non, cree un nouveau timer
        (bind _returnvalue (`KismetSystemLibrary.K2_SetTimerDelegate` (`|CreateDelegate` :!event `Timer`) 0.1 true))
        (set `self.Timer Handle` _returnvalue)
        (`KismetSystemLibrary.PrintString` "Timer Created" false)))))

(event `self.Box.OnComponentEndOverlap`
  (params (OverlappedComponent :type "PrimitiveComponent Object Reference") (OtherActor :type "Actor Object Reference") (OtherComp :type "PrimitiveComponent Object Reference") (OtherBodyIndex :type Integer))
  ; Check we've ovelapped with player (Je sais pas comment traduire x2)
  (if (`self.IsPlayerActor ?` OtherActor)
    (`KismetSystemLibrary.PrintString` "Sttop Checking" false)
    ; Pause le timer
    (`KismetSystemLibrary.K2_PauseTimerHandle` (`self.Timer Handle`))))

(fn `BP_CameraTrigger_AutoGenFunc`)

(fn `BP_CameraTrigger_AutoGenFunc1`)

(fn `IsPlayerActor ?`
  (params (A :type "Object Object Reference"))
  (returns (ReturnValue :type Boolean))
  (return (== A (`GameplayStatics.GetPlayerCharacter` 0))))

(fn `UserConstructionScript`)